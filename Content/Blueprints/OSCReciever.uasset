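; Receives OSC messages over the network to drive the two paddles of what appears to be a Pong game.
; On BeginPlay it starts two OSC servers on a hardcoded IP, one port each, and binds their message-received events.
; Each handler remaps the message's first float from 0–1 to an inverted X position, moving the Enemy_AI actor or the Pong_Player's Cube.
; Message addresses do not affect routing.
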(event Custom|OSCMessage
  (params (Message :type OSC%20Message%20Structure%20%28by%20ref%29) (IPAddress :type String) (Port :type Integer))
  (bind _returnvalue (Class|OSCManager|GetOSCMessageAddress Message))
  (Class|OSCManager|GetOSCAddressFullPath _returnvalue)
  (bind _value (Class|OSCManager|GetFloat Message))
  (bind _returnvalue_2 (Actor|GetActorOfClass "/Game/Blueprints/Enemy_AI.Enemy_AI_C"))
  (Transformation|SetActorTransform _returnvalue_2 (Math|Transform|MakeTransform (Math|Vector|MakeVector (Math|Float|MapRangeClamped _value 0.0 1.0 4e+02 -4e+02) 0.0 1.2e+02) "0, 0, 0" "1,1,1")))

(event Custom|OSCMessage2
  (params (Message :type OSC%20Message%20Structure%20%28by%20ref%29) (IPAddress :type String) (Port :type Integer))
  (bind _value (Class|OSCManager|GetFloat Message))
  (bind _returnvalue (Actor|GetActorOfClass "/Game/Blueprints/Pong_Player.Pong_Player_C"))
  (Transformation|SetWorldLocation (Variables|/Game/Blueprints/Pong_Player.Pong_Player_C|GetCube _returnvalue) (Math|Vector|MakeVector (Math|Float|MapRangeClamped _value 0.0 1.0 4e+02 -4e+02) -7e+02 1.2e+02) false false))

(event EventBeginPlay
  (bind _returnvalue (Class|OSCManager|CreateOSCServer "192.168.1.208" 8080 false true "" 0))
  (bind _output_get (Variables|Default|SetOSCReciever _returnvalue))
  (EventDispatchers|UnbindallEventsfromOnOscBundleReceived _output_get)
  (EventDispatchers|BindEventtoOnOscMessageReceived _output_get (EventDispatchers|CreateEvent :!event Custom|OSCMessage))
  (bind _returnvalue_2 (Class|OSCManager|CreateOSCServer "192.168.1.208" 8020 false true "" 0))
  (bind _output_get_2 (Variables|Default|SetOSCReciever2 _returnvalue_2))
  (EventDispatchers|UnbindallEventsfromOnOscBundleReceived _output_get_2)
  (EventDispatchers|BindEventtoOnOscMessageReceived _output_get_2 (EventDispatchers|CreateEvent :!event Custom|OSCMessage2)))

(fn ConstructionScript)