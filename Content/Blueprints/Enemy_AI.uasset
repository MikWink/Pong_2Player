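; Enemy AI actor with a Cube component, apparently meant to follow the Ball actor along the X axis.
; BeginPlay sets the tick interval, and each Tick looks up the Ball, caches its Sphere's relative location and calls Move.
; Move is empty: the MoveComponentTo that would slide the Cube to the ball's X at a fixed Y is disconnected and never runs.
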(event Custom|Move)

(event EventBeginPlay
  (Actor|Tick|SetActorTickInterval (Variables|Default|GetTickInterval)))

(event Collision|EventActorBeginOverlap
  (params (OtherActor :type Actor%20Object%20Reference)))

(event EventTick
  (params (DeltaSeconds :type Float%20%28single-precision%29))
  (bind _returnvalue (Actor|GetActorOfClass "/Game/Blueprints/Ball.Ball_C"))
  (Variables|Default|SetBall_Loc (Variables|/Script/Engine.SceneComponent|GetRelativeLocation (Variables|/Game/Blueprints/Ball.Ball_C|GetSphere _returnvalue)))
  (CallFunction|Move))

(fn ConstructionScript)